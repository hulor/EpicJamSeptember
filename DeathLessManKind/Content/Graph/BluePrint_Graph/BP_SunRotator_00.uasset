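; BP_SunRotator_00 is an actor that continuously spins its SunCenter component around the yaw axis, apparently to orbit a sun.
; BeginPlay zeroes a stored rotation, then each Tick adds a yaw step of delta time times ZRotationSpeed and applies it as SunCenter's relative rotation.
; An alternative AddLocalRotation node remains in the graph but never runs.
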(event EventTick
  (params (DeltaSeconds :type Float%20%28single-precision%29))
  (bind _previous_rot (Variables|Default|GetPrevious%20Rot))
  (bind _z_rotation_speed (Variables|Default|GetZ%20Rotation%20Speed))
  (bind _returnvalue (* DeltaSeconds _z_rotation_speed))
  (bind _returnvalue_2 (Class|KismetMathLibrary|MakeRot 0.0 _returnvalue 0.0))
  (bind _returnvalue_3 (Math|Rotator|CombineRotators _previous_rot _returnvalue_2))
  (Transformation|SetRelativeRotation (Variables|Default|GetSun_Center) _returnvalue_3 false)
  (Variables|Default|SetPreviousRot _returnvalue_3))

(event EventBeginPlay
  (Variables|Default|SetPreviousRot "0, 0, 0"))

(fn ConstructionScript)